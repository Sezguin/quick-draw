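; GM_Duel is a duel game mode that times the signal to draw after a random wait.
; Tick accumulates elapsed time and, once the Intro phase reaches the round start time, switches to Wait and starts a random delay.
; When the delay ends, it sets the Draw phase and shows the BP_Exclamation actor found at BeginPlay.
; Only the Intro phase has Tick logic, with debug prints along the way.
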(event EventBeginPlay
  (bind _returnvalue (Actor|GetActorOfClass "/Game/Blueprints/BP_Exclamation.BP_Exclamation_C"))
  (Variables|Default|SetExclamationRef _returnvalue))

(event EventTick
  (params (DeltaSeconds :type Float%20%28single-precision%29))
  (Variables|Default|SetElapsedTime (+ DeltaSeconds (Variables|Default|GetElapsedTime)))
  (switch Utilities|FlowControl|Switch|SwitchonE_Phase (Variables|Default|GetPhase)
    (:NewEnumerator0
      (if (>= (Variables|Default|GetElapsedTime) (Variables|Default|GetRoundStartTime))
        (Development|PrintString "Wait")
        (Variables|Default|SetPhase "NewEnumerator1")
        (Utilities|FlowControl|Delay (Math|Random|RandomFloatinRange (Variables|Default|GetMinDrawDelay) (Variables|Default|GetMaxDrawDelay)))
        (Variables|Default|SetPhase "NewEnumerator2")
        (Utilities|IsValid (Variables|Default|GetExclamationRef)
          (:Is%20Valid
            (Default|SetVisibility (Variables|Default|GetExclamationRef) true))
          (:Is%20Not%20Valid
            (Development|PrintString "Exclamation not found!")))
        (else
          (Development|PrintString "Time not met"))))))

(fn ConstructionScript)